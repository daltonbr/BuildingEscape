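; Door actor that animates its SMDoor component open by rotating it around the yaw axis.
; While IsOpen is false, Tick accumulates ElapsedTime and samples OpenYawCurve at that time normalized by LengthOfCurve to set relative yaw.
; Once the time exceeds LengthOfCurve, IsOpen becomes true and rotation stops.
; The graph has no trigger or closing logic.
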(event `self.ReceiveTick`
  (params (DeltaSeconds :type "Float (single-precision)"))
  (if (not (`self.bIsOpen`))
    (bind _output_get (set `self.ElapsedTime` (+ DeltaSeconds (`self.ElapsedTime`))))
    (if (> _output_get (`self.LengthOfCurve`))
      (set `self.bIsOpen` true)
      (else
        (`SceneComponent.K2_SetRelativeRotation` (`self.SM_Door`) (`KismetMathLibrary.MakeRotator` 0.0 0.0 (`CurveFloat.GetFloatValue` (`self.OpenYawCurve`) (/ (`self.ElapsedTime`) (`self.LengthOfCurve`)))) false false)))))

(fn `UserConstructionScript`)